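; Boost is a pickup-style actor Blueprint that animates its MovableScene component with a continuous spin and vertical bob.
; Each Tick it yaws the component by RotationSpeed scaled by world delta time.
; It also accumulates time and uses a modulo of Period to build a linear triangle wave, moving the relative Z between the lower and upper height bounds.
; No overlap or boost effect logic is present here.
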(event EventTick
  (params (DeltaSeconds :type Float%20%28single-precision%29))
  (bind _period (Variables|Default|Getperiod))
  (bind _returnvalue (/ _period 2.0))
  (Variables|Default|Settime (+ DeltaSeconds (Variables|Default|Gettime)))
  (Transformation|AddRelativeRotation (Variables|Default|GetMovableScene) (Math|Rotator|MakeRotator 0.0 0.0 (* (Variables|Default|GetrotationSpeed) (Utilities|Time|GetWorldDeltaSeconds))) false false)
  (if (< (Math|Float|%(Float) (Variables|Default|Gettime) (Variables|Default|Getperiod)) _returnvalue)
    (Variables|Default|SettargetZ (+ (Variables|Default|GethightLowerBound) (* (- (Variables|Default|GethightUpperBound) (Variables|Default|GethightLowerBound)) (/ (Math|Float|%(Float) (Variables|Default|Gettime) _returnvalue) _returnvalue))))
    (else
      (Variables|Default|SettargetZ (- (Variables|Default|GethightUpperBound) (* (- (Variables|Default|GethightUpperBound) (Variables|Default|GethightLowerBound)) (/ (Math|Float|%(Float) (Variables|Default|Gettime) _returnvalue) _returnvalue))))))
  (Transformation|SetRelativeLocation (Variables|Default|GetMovableScene) (Math|Vector|MakeVector 0.0 0.0 (Variables|Default|GettargetZ)) false false))

(fn ConstructionScript)