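; BoostSpawnPoint is a location in the waves level where boost pickups spawn.
; It caches the player character and waves game mode on BeginPlay and offers a check that the player is at least a given distance away.
; SpawnBoost creates the given boost class at its transform, links it back to the point, and records the type and occupied state.
; BoostCollected frees the point and reports the boost type to the game mode.
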(event EventBeginPlay
  (bind _asbp_player_character (Utilities|Casting|CastToBP_PlayerCharacter (Game|GetPlayerCharacter 0)))
  (Variables|Default|SetplayerCharacter _asbp_player_character)
  (bind _asbp_waves_level_game_mode (Utilities|Casting|CastToBP_WavesLevelGameMode (Game|GetGameMode)))
  (Variables|Default|SetgameMode _asbp_waves_level_game_mode))

(fn ConstructionScript)

(fn IsPlayerFarEnoughtoSpawn
  (params (distance :type Float%20%28single-precision%29))
  (return (>= (Math|Vector|Distance(Vector) (Transformation|GetActorLocation) (Transformation|GetActorLocation (Variables|Default|GetplayerCharacter))) distance)))

(fn SpawnBoost
  (params (boostType :type Boost%20Class%20Reference))
  (bind _returnvalue (Game|SpawnActorfromClass boostType (Transformation|GetActorTransform) "Undefined" 0 0))
  (Variables|/Game/Blueprints/Boosts/Boost.Boost_C|SetspawnPoint _returnvalue self)
  (Variables|Default|SetisBoostSpawned true)
  (Variables|Default|SetboostType boostType))

(fn BoostCollected
  (Variables|Default|SetisBoostSpawned false)
  (Default|BoostCollected (Variables|Default|GetgameMode) (Variables|Default|GetboostType)))