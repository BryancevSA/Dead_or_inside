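; Burst shotgun weapon, a gun Blueprint that combines an angled two-bullet spread with a timed burst of straight shots.
; Fire checks cooldown, ammo and any running burst, then spends one ammo, plays a sound, spawns two side bullets yawed either way and arms the burst.
; Tick spawns the burst bullets at a fixed interval.
; Every bullet takes the attach parent's class as its friendly class.
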(event EventTick
  (params (DeltaSeconds :type Float%20%28single-precision%29))
  (|CallParentFunction DeltaSeconds)
  (if (> (Variables|Default|GetburstShotsLeft) 0)
    (if (> (Variables|Default|GetburstIntervalTimeLeft) 0.0)
      (Variables|Default|SetburstIntervalTimeLeft (- (Variables|Default|GetburstIntervalTimeLeft) (Utilities|Time|GetWorldDeltaSeconds)))
      (else
        (Variables|Default|SetburstIntervalTimeLeft (Variables|Default|GetburstIntervalDuration))
        (Math|Integer|DecrementInt (Variables|Default|GetburstShotsLeft)
          (:%20%20
            (bind _returnvalue (Game|SpawnActorfromClass (Variables|Default|GetburstBullet) (Transformation|GetWorldTransform (Variables|Default|GetFireDirection)) "Undefined" 0 0))
            (Utilities|IsValid _returnvalue
              (:Is%20Valid
                (Variables|/Game/Blueprints/Weapon/Bullets/BP_Bullet.BP_Bullet_C|SetfriendlyActorClass _returnvalue (Utilities|GetClass (Actor|GetAttachParentActor)))))))))))

(event EventFire
  (bind _returnvalue (Actor|GetAttachParentActor))
  (bind _deviationangle (Variables|Default|GetdeviationAngle))
  (bind _firedirection (Variables|Default|GetFireDirection))
  (bind _sidebullet (Variables|Default|GetsideBullet))
  (bind _returnvalue_2 (Utilities|GetClass _returnvalue))
  (bind _returnvalue_3 (Transformation|GetWorldTransform _firedirection))
  (if (and (and (<= (Variables|Default|GetcooldownLeft) 0.0) (<= (Variables|Default|GetburstShotsLeft) 0)) (> (Variables|Default|Getammo) 0))
    (Audio|PlaySound2D "/Game/Assets/Sounds/GunSounds/RifleBurstCue.RifleBurstCue" 0.1 1.0 0.0 0 0)
    (Math|Integer|DecrementInt (Variables|Default|Getammo)
      (:%20%20
        (Variables|Default|SetcooldownLeft (Variables|Default|GetcooldownDuration))
        (Variables|Default|SetburstIntervalTimeLeft 0.0)
        (Variables|Default|SetburstShotsLeft (Variables|Default|GetburstLength))
        (Utilities|FlowControl|Sequence
          (:then_0
            (bind _returnvalue_4 (Game|SpawnActorfromClass _sidebullet _returnvalue_3 "Undefined" 0 0))
            (Utilities|IsValid _returnvalue_4
              (:Is%20Valid
                (Variables|/Game/Blueprints/Weapon/Bullets/BP_Bullet.BP_Bullet_C|SetfriendlyActorClass _returnvalue_4 _returnvalue_2)
                (Transformation|AddActorLocalRotation _returnvalue_4 (Math|Rotator|MakeRotator 0.0 0.0 _deviationangle) false false))))
          (:then_1
            (bind _returnvalue_5 (Game|SpawnActorfromClass _sidebullet _returnvalue_3 "Undefined" 0 0))
            (Utilities|IsValid _returnvalue_5
              (:Is%20Valid
                (Variables|/Game/Blueprints/Weapon/Bullets/BP_Bullet.BP_Bullet_C|SetfriendlyActorClass _returnvalue_5 _returnvalue_2)
                (Transformation|AddActorLocalRotation _returnvalue_5 (Math|Rotator|MakeRotator 0.0 0.0 (* -1 _deviationangle)) false false)
                (Development|PrintString (Utilities|String|ToString(Integer) (Variables|Default|Getammo)))))))))))

(fn ConstructionScript
  (|CallParentFunction)
  (CallFunction|InitGunParams 1.0 10 2 "Burst shotgun"))