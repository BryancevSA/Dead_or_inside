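; BP_ShotGun is the shotgun weapon, a child gun Blueprint that sets its cooldown, ammo and name through InitGunParams in the construction script.
; When off cooldown with ammo left, Fire spends one round, plays a sound and spawns a single BP_ShotgunBullet at the FireDirection transform.
; The bullet's FriendlyActorClass is set to the class of the gun's attach parent, and remaining ammo is printed for debugging.
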(event EventFire
  (if (and (<= (Variables|Default|GetcooldownLeft) 0.0) (> (Variables|Default|Getammo) 0))
    (Math|Integer|DecrementInt (Variables|Default|Getammo)
      (:%20%20
        (Variables|Default|SetcooldownLeft (Variables|Default|GetcooldownDuration))
        (Audio|PlaySound2D "/Game/Assets/Sounds/GunSounds/ShotgunCue.ShotgunCue" 0.1 1.0 0.0 0 0)
        (bind _returnvalue (Game|SpawnActorfromClass "/Game/Blueprints/Weapon/Bullets/BP_ShotgunBullet.BP_ShotgunBullet_C" (Transformation|GetWorldTransform (Variables|Default|GetFireDirection)) "Undefined" 0 0))
        (Utilities|IsValid _returnvalue
          (:Is%20Valid
            (Variables|/Game/Blueprints/Weapon/Bullets/BP_Bullet.BP_Bullet_C|SetfriendlyActorClass _returnvalue (Utilities|GetClass (Actor|GetAttachParentActor)))
            (Development|PrintString (Utilities|String|ToString(Integer) (Variables|Default|Getammo)))))))))

(event EventTick
  (params (DeltaSeconds :type Float%20%28single-precision%29))
  (|CallParentFunction DeltaSeconds))

(fn ConstructionScript
  (|CallParentFunction)
  (CallFunction|InitGunParams 1.0 15 0 "Shotgun"))