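; BP_Gun is a gun Blueprint that holds ammo, gun type and fire cooldown state.
; InitGunParams sets the cooldown duration, starting ammo and type, and BeginPlay starts the cooldown at its full duration.
; Tick counts the cooldown down by world delta time, but only while ammo remains.
; The Fire event is empty, so this file contains no shooting, ammo use or cooldown reset.
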(event Custom|Fire)

(event EventBeginPlay
  (Variables|Default|SetcooldownLeft (Variables|Default|GetcooldownDuration)))

(event EventTick
  (params (DeltaSeconds :type Float%20%28single-precision%29))
  (if (and (> (Variables|Default|GetcooldownLeft) 0.0) (> (Variables|Default|Getammo) 0))
    (Variables|Default|SetcooldownLeft (- (Variables|Default|GetcooldownLeft) (Utilities|Time|GetWorldDeltaSeconds)))))

(fn ConstructionScript)

(fn InitGunParams
  (params (cooldownDuration :type Float%20%28single-precision%29) (initialAmmo :type Integer) (gunType :type Integer))
  (Variables|Default|SetcooldownDuration cooldownDuration)
  (Variables|Default|Setammo initialAmmo)
  (Variables|Default|SetgunType gunType))