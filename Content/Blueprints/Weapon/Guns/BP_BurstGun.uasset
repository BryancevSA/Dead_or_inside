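; BP_BurstGun is a gun that fires a burst of bullets per trigger pull, using one ammo per burst.
; Fire checks cooldown, ammo and any running burst, then plays a sound, prints remaining ammo and arms the burst counter.
; Tick calls the parent, then spawns bullets from FireDirection at a fixed interval until the burst ends.
; The construction script sets cooldown, starting ammo and gun type through InitGunParams.
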(event EventTick
  (params (DeltaSeconds :type Float%20%28single-precision%29))
  (|CallParentFunction DeltaSeconds)
  (if (> (Variables|Default|GetburstShotsLeft) 0)
    (if (> (Variables|Default|GetburstIntervalTimeLeft) 0.0)
      (Variables|Default|SetburstIntervalTimeLeft (- (Variables|Default|GetburstIntervalTimeLeft) (Utilities|Time|GetWorldDeltaSeconds)))
      (else
        (Variables|Default|SetburstIntervalTimeLeft (Variables|Default|GetburstIntervalDuration))
        (Math|Integer|DecrementInt (Variables|Default|GetburstShotsLeft)
          (:%20%20
            (Game|SpawnActorfromClass (Variables|Default|GetburstBullet) (Transformation|GetWorldTransform (Variables|Default|GetFireDirection)) "Undefined" 0 0)))))))

(event EventFire
  (if (and (and (<= (Variables|Default|GetcooldownLeft) 0.0) (<= (Variables|Default|GetburstShotsLeft) 0)) (> (Variables|Default|Getammo) 0))
    (Audio|PlaySound2D "/Game/Assets/Sounds/GunSounds/RifleBurstCue.RifleBurstCue" 0.1 1.0 0.0 0 0)
    (Math|Integer|DecrementInt (Variables|Default|Getammo)
      (:%20%20
        (Variables|Default|SetcooldownLeft (Variables|Default|GetcooldownDuration))
        (Variables|Default|SetburstIntervalTimeLeft 0.0)
        (Variables|Default|SetburstShotsLeft (Variables|Default|GetburstLength))
        (Development|PrintString (Utilities|String|ToString(Integer) (Variables|Default|Getammo)))))))

(fn ConstructionScript
  (|CallParentFunction)
  (CallFunction|InitGunParams 1.0 2))