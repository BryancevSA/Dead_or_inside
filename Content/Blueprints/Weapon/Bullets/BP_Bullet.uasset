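; BP_Bullet is a projectile actor that damages zombies, soldiers or the player on overlap.
; Speed, range and damage are set through InitParams, and Tick teleports it along its forward vector, destroying it once it exceeds max distance from its start.
; Overlaps with other bullets, spawn points, attack colliders, boosts and its friendly actor class are ignored; any other overlap destroys it, calling GetDamage on those character types.
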(event EventBeginPlay
  (Variables|Default|SetstartLocation (Transformation|GetActorLocation)))

(event EventTick
  (params (DeltaSeconds :type Float%20%28single-precision%29))
  (Transformation|Teleport (+ (Transformation|GetActorLocation) (* (* (Transformation|GetActorForwardVector) (Variables|Default|Getspeed)) (Utilities|Time|GetWorldDeltaSeconds))) (Transformation|GetActorRotation))
  (if (> (Math|Vector|Distance(Vector) (Variables|Default|GetstartLocation) (Transformation|GetActorLocation)) (Variables|Default|GetmaxDistance))
    (Actor|DestroyActor)))

(event Collision|EventActorBeginOverlap
  (params (OtherActor :type Actor%20Object%20Reference))
  (bind _returnvalue (Utilities|GetClass OtherActor))
  (if (not (or (Utilities|ClassIsChildOf _returnvalue "BP_Bullet_C") (or (Utilities|ClassIsChildOf _returnvalue "/Game/Blueprints/GameManagement/BP_ZombieSpawnPoint.BP_ZombieSpawnPoint_C") (or (Utilities|ClassIsChildOf _returnvalue "/Game/Blueprints/Bots/BP_Attack_Collider.BP_Attack_Collider_C") (or (Utilities|ClassIsChildOf _returnvalue "/Game/Blueprints/Boosts/Boost.Boost_C") (Utilities|ClassIsChildOf _returnvalue (Variables|Default|GetfriendlyActorClass)))))))
    (Actor|DestroyActor)
    (bind _asbp_zombie_character (Utilities|Casting|CastToBP_ZombieCharacter OtherActor)
      (:then
        (Default|GetDamage _asbp_zombie_character (Variables|Default|Getdamage)))
      (:CastFailed
        (bind _asbp_soldier (Utilities|Casting|CastToBP_Soldier OtherActor)
          (:then
            (Default|GetDamage _asbp_soldier (Variables|Default|Getdamage)))
          (:CastFailed
            (bind _asbp_player_character (Utilities|Casting|CastToBP_PlayerCharacter OtherActor))
            (Default|GetDamage _asbp_player_character (Variables|Default|Getdamage))))))))

(fn ConstructionScript)

(fn InitParams
  (params (speed :type Float%20%28single-precision%29) (maxDistance :type Float%20%28single-precision%29) (damage :type Float%20%28single-precision%29))
  (Variables|Default|Setspeed speed)
  (Variables|Default|SetmaxDistance maxDistance)
  (Variables|Default|Setdamage damage))