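; BP_Soldier is an enemy bot soldier that carries a gun, takes damage and dies, and caches the waves level game mode.
; On BeginPlay it spawns a gun class looked up by GunType, attaches it to GunSocket and initializes its HP bar widget.
; Shoot fires that gun.
; GetDamage reveals and updates the bar, then at zero HP flags the death animation and destroys gun and soldier after a delay.
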(event Custom|Shoot
  (Default|Fire (Variables|Default|GetcurrentGun)))

(event Custom|Get%20Damage
  (params (damage :type Float%20%28single-precision%29))
  (bind _myhpbar (Variables|Default|GetMyHpBar))
  (Widget|SetVisibility _myhpbar "Visible")
  (if (> (Variables|Default|Gethp) 0.0)
    (bind _output_get (Variables|Default|Sethp (Math|Float|Max(Float) (- (Variables|Default|Gethp) damage) 0.0)))
    (bind _output_get_2 (Variables|/Game/UI/Widgets/EnemyHPBar.EnemyHPBar_C|SetHP _myhpbar _output_get))
    (if (== _output_get_2 0.0)
      (bind _asbp_anim_soldier (Utilities|Casting|CastToBP_Anim_Soldier (Components|SkeletalMesh|GetAnimInstance (Variables|Character|GetMesh))))
      (Variables|/Game/Blueprints/Bots/Soldiers/BP_Anim_Soldier.BP_Anim_Soldier_C|SetIs%20Dead _asbp_anim_soldier true)
      (Utilities|FlowControl|Delay 2.0)
      (Actor|DestroyActor (Variables|Default|GetcurrentGun))
      (Actor|DestroyActor))))

(event EventBeginPlay
  (bind _asbp_game_mode (Utilities|Casting|CastToBP_WavesLevelGameMode (Game|GetGameMode)))
  (Variables|Default|SetgameMode _asbp_game_mode)
  (CallFunction|SelectGun (Variables|Default|GetgunType))
  (bind _asenemy_hpbar (Utilities|Casting|CastToEnemyHPBar (UserInterface|GetUserWidgetObject (Variables|Default|GetHPBar))))
  (bind _output_get (Variables|Default|SetMyHpBar _asenemy_hpbar))
  (Variables|/Game/UI/Widgets/EnemyHPBar.EnemyHPBar_C|SetmaxHP _output_get (Variables|Default|Gethp)))

(fn ConstructionScript)

(fn SelectGun
  (params (gunNumber :type Integer))
  (Utilities|IsValid (Variables|Default|GetcurrentGun)
    (:Is%20Valid
      (Actor|DestroyActor (Variables|Default|GetcurrentGun)))
    (:Is%20Not%20Valid
      _))
  (bind _returnvalue (Game|SpawnActorfromClass (.Value (Utilities|Map|Find (Variables|Default|Getguns) gunNumber)) (Math|Transform|MakeTransform "0, 0, 0" "0, 0, 0" "1,1,1") "Undefined" 0 0))
  (Transformation|AttachComponentToComponent _returnvalue (Variables|Character|GetMesh) "GunSocket" "KeepRelative" "KeepRelative" "KeepRelative" true)
  (Variables|Default|SetcurrentGun _returnvalue))