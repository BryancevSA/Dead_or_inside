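; BP_ZombieCharacter is a zombie bot character that chases the player and can be killed by damage.
; BeginPlay caches the first player's BP_PlayerCharacter, and every Tick feeds movement input at half scale straight toward that player's location, without pathfinding.
; GetDamage subtracts from Hp, clamps it at zero and destroys the actor when it runs out.
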(event EventBeginPlay
  (bind _asbp_player_character (Utilities|Casting|CastToBP_PlayerCharacter (Game|GetPlayerCharacter 0)))
  (Variables|Default|SetplayerCharacter _asbp_player_character))

(event EventTick
  (params (DeltaSeconds :type Float%20%28single-precision%29))
  (Pawn|Input|AddMovementInput (Class|KismetMathLibrary|VectorNormalUnsafe (- (Transformation|GetActorLocation (Variables|Default|GetplayerCharacter)) (Transformation|GetActorLocation))) 0.5 false))

(fn ConstructionScript)

(fn GetDamage
  (params (damage :type Float%20%28single-precision%29))
  (bind _output_get (Variables|Default|Sethp (Math|Float|Max(Float) (- (Variables|Default|Gethp) damage) 0.0)))
  (if (== _output_get 0.0)
    (Actor|DestroyActor)))