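; Shotgun Blueprint, a gun subclass that fires a three-bullet horizontal spread when the Fire input is pressed.
; Each shot spawns bullets at the FireDirection transform: one straight ahead and two yawed by separately randomized angles, the second negated to mirror the spread.
; A cooldown counted down on Tick gates firing.
; The construction script runs the parent's, then sets the cooldown duration and gun type.
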(event EventTick
  (params (DeltaSeconds :type Float%20%28single-precision%29))
  (if (> (Variables|Default|GetcooldownLeft) 0.0)
    (Variables|Default|SetcooldownLeft (- (Variables|Default|GetcooldownLeft) (Utilities|Time|GetWorldDeltaSeconds)))))

(event Input|ActionEvents|InputActionFire
  (params (Key :type Key%20Structure :default "None"))
  (bind _firedirection (Variables|Default|GetFireDirection))
  (bind _mindeviationangle (Variables|Default|GetminDeviationAngle))
  (bind _maxdeviationangle (Variables|Default|GetmaxDeviationAngle))
  (bind _returnvalue (Transformation|GetWorldTransform _firedirection))
  (bind _returnvalue_2 (Math|Random|RandomFloatinRange _mindeviationangle _maxdeviationangle))
  (:Pressed
    (if (<= (Variables|Default|GetcooldownLeft) 0.0)
      (Variables|Default|SetcooldownLeft (Variables|Default|GetcooldownDuration))
      (Utilities|FlowControl|Sequence
        (:then_0
          (bind _returnvalue_3 (Game|SpawnActorfromClass "/Game/Blueprints/Guns/BP_ShotgunBullet.BP_ShotgunBullet_C" _returnvalue "Undefined" 0 0))
          (Utilities|IsValid _returnvalue_3
            (:Is%20Valid
              (Transformation|AddActorLocalRotation _returnvalue_3 (Math|Rotator|MakeRotator 0.0 0.0 _returnvalue_2) false false))))
        (:then_1
          (Game|SpawnActorfromClass "/Game/Blueprints/Guns/BP_ShotgunBullet.BP_ShotgunBullet_C" _returnvalue "Undefined" 0 0))
        (:then_2
          (bind _returnvalue_4 (Game|SpawnActorfromClass "/Game/Blueprints/Guns/BP_ShotgunBullet.BP_ShotgunBullet_C" _returnvalue "Undefined" 0 0))
          (Utilities|IsValid _returnvalue_4
            (:Is%20Valid
              (Transformation|AddActorLocalRotation _returnvalue_4 (Math|Rotator|MakeRotator 0.0 0.0 (* _returnvalue_2 -1.0)) false false))))))))

(fn ConstructionScript
  (|CallParentFunction)
  (Variables|Default|SetcooldownDuration 1.0)
  (Variables|Default|SetGunType 1))