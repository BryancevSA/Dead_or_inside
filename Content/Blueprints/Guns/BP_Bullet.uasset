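; BP_Bullet is a gun projectile actor that damages zombies on contact.
; Each tick it teleports forward along its facing at Speed scaled by delta time, then destroys itself once it travels beyond MaxDistance from its spawn location.
; Overlapping a BP_ZombieCharacter destroys the bullet and calls GetDamage on the zombie, while other overlapping actors are ignored.
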(event EventBeginPlay
  (Variables|Default|SetstartLocation (Transformation|GetActorLocation)))

(event EventTick
  (params (DeltaSeconds :type Float%20%28single-precision%29))
  (Transformation|Teleport (+ (Transformation|GetActorLocation) (* (* (Transformation|GetActorForwardVector) (Variables|Default|Getspeed)) (Utilities|Time|GetWorldDeltaSeconds))) (Transformation|GetActorRotation))
  (if (> (Math|Vector|Distance(Vector) (Variables|Default|GetstartLocation) (Transformation|GetActorLocation)) (Variables|Default|GetmaxDistance))
    (Actor|DestroyActor)))

(event Collision|EventActorBeginOverlap
  (params (OtherActor :type Actor%20Object%20Reference))
  (bind _asbp_zombie_character (Utilities|Casting|CastToBP_ZombieCharacter OtherActor))
  (Actor|DestroyActor)
  (Default|GetDamage _asbp_zombie_character (Variables|Default|Getdamage)))

(fn ConstructionScript)