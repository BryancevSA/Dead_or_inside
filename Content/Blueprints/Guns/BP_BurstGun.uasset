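; BP_BurstGun is a gun Blueprint that fires a timed burst of BP_BurstBullet projectiles each time it is triggered.
; Fire starts the cooldown and queues a burst, but only when the cooldown has elapsed and no burst is in progress.
; Tick counts down the cooldown and the interval between shots, spawning each bullet at the FireDirection component's transform.
; The construction script calls the parent's, then sets the cooldown duration and gun type.
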(event EventTick
  (params (DeltaSeconds :type Float%20%28single-precision%29))
  (Utilities|FlowControl|Sequence
    (:then_0
      (if (> (Variables|Default|GetcooldownLeft) 0.0)
        (Variables|Default|SetcooldownLeft (- (Variables|Default|GetcooldownLeft) (Utilities|Time|GetWorldDeltaSeconds)))))
    (:then_1
      (if (> (Variables|Default|GetburstShotsLeft) 0)
        (if (> (Variables|Default|GetburstIntervalTimeLeft) 0.0)
          (Variables|Default|SetburstIntervalTimeLeft (- (Variables|Default|GetburstIntervalTimeLeft) (Utilities|Time|GetWorldDeltaSeconds)))
          (else
            (Variables|Default|SetburstIntervalTimeLeft (Variables|Default|GetburstIntervalDuration))
            (Math|Integer|DecrementInt (Variables|Default|GetburstShotsLeft)
              (:%20%20
                (Game|SpawnActorfromClass "/Game/Blueprints/Guns/BP_BurstBullet.BP_BurstBullet_C" (Transformation|GetWorldTransform (Variables|Default|GetFireDirection)) "Undefined" 0 0)))))))))

(event EventFire
  (if (and (<= (Variables|Default|GetcooldownLeft) 0.0) (<= (Variables|Default|GetburstShotsLeft) 0))
    (Utilities|FlowControl|Sequence
      (:then_0
        (Variables|Default|SetcooldownLeft (Variables|Default|GetcooldownDuration)))
      (:then_1
        (Variables|Default|SetburstIntervalTimeLeft 0.0)
        (Variables|Default|SetburstShotsLeft (Variables|Default|GetburstLength))))))

(fn ConstructionScript
  (|CallParentFunction)
  (Variables|Default|SetcooldownDuration 1.0)
  (Variables|Default|SetGunType 0))