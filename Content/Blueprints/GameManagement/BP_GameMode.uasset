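; Game mode for a zombie wave survival game with boost pickups, a saved wave record, HUD, pause and game-over menus.
; Per-spawner maps hold fast and slow zombie counts, which grow at random indices each time the last zombie dies and a new wave spawns.
; A Tick-driven cooldown spawns a random under-cap boost type at a free point far enough from the player.
; Player death saves any new record.
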(event Custom|Player%20Death
  (bind _returnvalue (Game|GetPlayerController 0))
  (bind _savegame (Variables|Default|GetSaveGame))
  (Variables|Default|SetisGameOver true)
  (if (> (Variables|Default|GetcurrentWave) (Variables|/Game/Blueprints/GameManagement/SaveGame.SaveGame_C|GetWaveRecord (Variables|Default|GetSaveGame)))
    (Variables|/Game/Blueprints/GameManagement/SaveGame.SaveGame_C|SetWaveRecord _savegame (Variables|Default|GetcurrentWave))
    (SaveGame|SaveGametoSlot _savegame "SaveDefault"))
  (Variables|/Script/Engine.PlayerController|SetbShowMouseCursor _returnvalue true)
  (bind _returnvalue_2 (UserInterface|CreateWidget "/Game/UI/Widgets/GameOverMenu.GameOverMenu_C" _returnvalue))
  (UserInterface|Viewport|AddtoViewport _returnvalue_2 0)
  (Input|SetInputModeUIOnly _returnvalue _returnvalue_2 "DoNotLock"))

(event Custom|Pause%20Game
  (Utilities|IsValid (Variables|Default|GetPauseMenu)
    (:Is%20Valid
      _)
    (:Is%20Not%20Valid
      (bind _returnvalue (UserInterface|CreateWidget "/Game/UI/Widgets/PauseMenu.PauseMenu_C"))
      (Variables|Default|SetPauseMenu _returnvalue)))
  (if (not (Game|IsGamePaused))
    (Game|SetGamePaused true)
    (UserInterface|Viewport|AddtoViewport (Variables|Default|GetPauseMenu) 0)
    (Input|SetInputModeUIOnly (Game|GetPlayerController 0) (Variables|Default|GetPauseMenu) "DoNotLock")))

(event EventBeginPlay
  (bind _returnvalue (SaveGame|LoadGamefromSlot "SaveDefault"))
  (bind _assave_game (Utilities|Casting|CastToSaveGame _returnvalue)
    (:then
      (Variables|Default|SetSaveGame _assave_game))
    (:CastFailed
      (bind _returnvalue_2 (SaveGame|CreateSaveGameObject "/Game/Blueprints/GameManagement/SaveGame.SaveGame_C"))
      (bind _output_get (Variables|Default|SetSaveGame _returnvalue_2))
      (SaveGame|SaveGametoSlot _output_get "SaveDefault")))
  (bind _outactors (Actor|GetAllActorsOfClass "/Game/Blueprints/GameManagement/BP_ZombieSpawnPoint.BP_ZombieSpawnPoint_C"))
  (bind _output_get_2 (Variables|Default|SetzombieSpawners _outactors))
  (for (_ _array_index) _output_get_2
    (Utilities|Map|Add (Variables|Default|GetfastZombiesToSpawn) _array_index 2)
    (Utilities|Map|Add (Variables|Default|GetslowZombiesToSpawn) _array_index 0)
    (Variables|Default|SetzombiesLeft (+ (Variables|Default|GetzombiesLeft) 2)))
  (bind _outactors_2 (Actor|GetAllActorsOfClass "/Game/Blueprints/Boosts/BoostSpawnPoint.BoostSpawnPoint_C"))
  (Variables|Default|SetboostSpawnPoints _outactors_2)
  (Utilities|FlowControl|Delay 5.0)
  (Variables|Default|SetboostSpawnTimeLeft (Variables|Default|GetboostSpawnCooldown))
  (CallFunction|SpawnAllZombies)
  (bind _returnvalue_3 (UserInterface|CreateWidget "/Game/UI/Widgets/HUD.HUD_C" (Game|GetPlayerController 0)))
  (UserInterface|Viewport|AddtoViewport _returnvalue_3 0))

(event EventTick
  (params (DeltaSeconds :type Float%20%28single-precision%29))
  (if (> (Utilities|Array|Length (Variables|Default|GetboostSpawnPoints)) 0)
    (if (> (Variables|Default|GetboostSpawnTimeLeft) 0.0)
      (Variables|Default|SetboostSpawnTimeLeft (- (Variables|Default|GetboostSpawnTimeLeft) (Utilities|Time|GetWorldDeltaSeconds)))
      (else
        (CallFunction|TrySpawnBoost)))))

(fn ConstructionScript)

(fn ZombieDied
  (Math|Integer|IncrementInt (Variables|Default|GetzombiesKilled)
    (:%20%20
      (bind _result (Math|Integer|DecrementInt (Variables|Default|GetzombiesLeft))
        (:%20%20
          (if (<= _result 0)
            (CallFunction|UpdateWave)))))))

(fn SpawnAllZombies
  (for (_array_element _array_index) (Variables|Default|GetzombieSpawners)
    (Default|SpawnZombies _array_element (.Value (Utilities|Map|Find (Variables|Default|GetfastZombiesToSpawn) _array_index)) (.Value (Utilities|Map|Find (Variables|Default|GetslowZombiesToSpawn) _array_index)))))

(fn UpdateWave
  (bind _zombiespawners (Variables|Default|GetzombieSpawners))
  (bind _zombiespawners_2 (Variables|Default|GetzombieSpawners))
  (bind _returnvalue (Utilities|Array|Length _zombiespawners))
  (bind _returnvalue_2 (Utilities|Array|Length _zombiespawners_2))
  (bind _returnvalue_3 (- _returnvalue 1))
  (bind _returnvalue_4 (- _returnvalue_2 1))
  (bind _returnvalue_5 (Math|Random|RandomIntegerinRange 0 _returnvalue_3))
  (bind _returnvalue_6 (Math|Random|RandomIntegerinRange 0 _returnvalue_4))
  (Math|Integer|IncrementInt (Variables|Default|GetcurrentWave)
    (:%20%20
      (for _index (range 0 (- (Variables|Default|GetfastZombiesToAddByWave) 1))
        (Utilities|Map|Add (Variables|Default|GetfastZombiesToSpawn) _returnvalue_6 (+ (.Value (Utilities|Map|Find (Variables|Default|GetfastZombiesToSpawn) _returnvalue_6)) 1)))
      (for _index_2 (range 0 (- (Variables|Default|GetslowZombiesToAddByWave) 1))
        (Utilities|Map|Add (Variables|Default|GetslowZombiesToSpawn) _returnvalue_5 (+ (.Value (Utilities|Map|Find (Variables|Default|GetslowZombiesToSpawn) _returnvalue_5)) 1)))
      (bind _values (Utilities|Map|Values (Variables|Default|GetfastZombiesToSpawn)))
      (for _array_element _values
        (Variables|Default|SetzombiesLeft (+ _array_element (Variables|Default|GetzombiesLeft))))
      (bind _values_2 (Utilities|Map|Values (Variables|Default|GetslowZombiesToSpawn)))
      (for _array_element_2 _values_2
        (Variables|Default|SetzombiesLeft (+ _array_element_2 (Variables|Default|GetzombiesLeft))))
      (CallFunction|SpawnAllZombies))))

(fn BoostCollected
  (params (boostType :type Boost%20Class%20Reference))
  (Math|Integer|DecrementInt (Utilities|Array|Get(acopy) (Variables|Default|GetboostSpawnedByType) (Utilities|Array|FindItem (Variables|Default|GetboostTypes) boostType))))

(fn TrySpawnBoost
  (for (_array_element _array_index) (Variables|Default|GetboostTypes)
    (if (< (Utilities|Array|Get(acopy) (Variables|Default|GetboostSpawnedByType) _array_index) (Utilities|Array|Get(acopy) (Variables|Default|GetboostMaxToSpawnByType) _array_index))
      (Utilities|Array|Add (LocalVariables|GetallowedTypesToSpawn) _array_element)))
  (if (> (Utilities|Array|Length (LocalVariables|GetallowedTypesToSpawn)) 0)
    (for _array_element_2 (Variables|Default|GetboostSpawnPoints)
      (bind _isfar (Default|IsPlayerFarEnoughtoSpawn _array_element_2 (Variables|Default|GetallowedBoostSpawnDistanceToPlayer)))
      (if (and _isfar (not (Variables|/Game/Blueprints/Boosts/BoostSpawnPoint.BoostSpawnPoint_C|GetisBoostSpawned _array_element_2)))
        (Utilities|Array|Add (LocalVariables|GetallowedSpawnPoints) _array_element_2)))
    (LocalVariables|SettypeToSpawn (.OutItem (Utilities|Array|Random (LocalVariables|GetallowedTypesToSpawn))))
    (Default|SpawnBoost (.OutItem (Utilities|Array|Random (LocalVariables|GetallowedSpawnPoints))) (LocalVariables|GettypeToSpawn))
    (Math|Integer|IncrementInt (Utilities|Array|Get(acopy) (Variables|Default|GetboostSpawnedByType) (Utilities|Array|FindItem (Variables|Default|GetboostTypes) (LocalVariables|GettypeToSpawn)))
      (:%20%20
        (Variables|Default|SetboostSpawnTimeLeft (Variables|Default|GetboostSpawnCooldown))))))