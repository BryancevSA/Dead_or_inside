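; Zombie spawn point actor that spawns queued fast and slow zombies at its own location.
; SpawnZombies adds the requested counts of each type to pending counters.
; Each Tick, when no zombie overlaps the point, it spawns one AI pawn, draining the fast queue before the slow one.
; The overlap check staggers spawns so each waits until the spot is clear.
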(event EventTick
  (params (DeltaSeconds :type Float%20%28single-precision%29))
  (if (== (Utilities|Array|Length (Collision|GetOverlappingActors "/Game/Blueprints/Bots/BP_ZombieCharacter.BP_ZombieCharacter_C" :!class /Script/Engine.Actor)) 0)
    (if (> (Variables|Default|GetfastZombiesToSpawnLeft) 0)
      (Math|Integer|DecrementInt (Variables|Default|GetfastZombiesToSpawnLeft)
        (:%20%20
          (AI|SpawnAIFromClass "/Game/Blueprints/Bots/BP_Zombie_Fast.BP_Zombie_Fast_C" 0 (Transformation|GetActorLocation) "0, 0, 0" false 0)))
      (elif (> (Variables|Default|GetslowZombiesToSpawnLeft) 0)
        (Math|Integer|DecrementInt (Variables|Default|GetslowZombiesToSpawnLeft)
          (:%20%20
            (AI|SpawnAIFromClass "/Game/Blueprints/Bots/BP_Zombie_Slow.BP_Zombie_Slow_C" 0 (Transformation|GetActorLocation) "0, 0, 0" false 0)))))))

(fn ConstructionScript)

(fn SpawnZombies
  (params (fastZombiesCount :type Integer) (slowZombiesCount :type Integer))
  (Variables|Default|SetfastZombiesToSpawnLeft (+ (Variables|Default|GetfastZombiesToSpawnLeft) fastZombiesCount))
  (Variables|Default|SetslowZombiesToSpawnLeft (+ (Variables|Default|GetslowZombiesToSpawnLeft) slowZombiesCount)))